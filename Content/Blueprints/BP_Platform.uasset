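; BP_Platform is a platform that disappears about two seconds after the third-person character touches it.
; An overlap on BoxColider applies a dynamic instance of the blue platform material to the Cube and starts a one-second Delay loop that increments a counter.
; After the first second the Cube's Color parameter turns red as a warning, and after the second the actor destroys itself.
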(event OnComponentBeginOverlap(BoxColider)
  (params (OverlappedComponent :type Primitive%20Component%20Object%20Reference) (OtherActor :type Actor%20Object%20Reference) (OtherComp :type Primitive%20Component%20Object%20Reference) (OtherBodyIndex :type Integer) (bFromSweep :type Boolean) (SweepResult :type Hit%20Result%20Structure%20%28by%20ref%29))
  ;[1 1 1] PLATFORM DESTROY AFTER 2 SCONDES
  (Utilities|Casting|CastToBP_ThirdPersonCharacter OtherActor)
  (Rendering|Material|CreateDynamicMaterialInstance (Variables|Default|GetCube) 0 "/Game/Material/MTL_PlatformBlue.MTL_PlatformBlue" "None" :!class /Script/Engine.PrimitiveComponent)
  (Variables|Default|SetCounter (+ (Variables|Default|GetCounter) 1.0) :!label _label)
  (Utilities|FlowControl|Delay 1.0)
  (if (== (Variables|Default|GetCounter) 1.0)
    (bind _returnvalue (Rendering|Material|CreateDynamicMaterialInstance (Variables|Default|GetCube) 0 "/Game/Material/MTL_PlatformBlue.MTL_PlatformBlue" "None" :!class /Script/Engine.PrimitiveComponent))
    (Rendering|Material|SetVectorParameterValue _returnvalue "Color" "(R=0.662500,G=0.000000,B=0.000000,A=1.000000)" :!class /Script/Engine.MaterialInstanceDynamic))
  (if (== (Variables|Default|GetCounter) 2.0)
    (Actor|DestroyActor)
    (else
      (goto _label))))

(event EventBeginPlay)

(event Collision|EventActorBeginOverlap
  (params (OtherActor :type Actor%20Object%20Reference)))

(event EventTick
  (params (DeltaSeconds :type Float%20%28single-precision%29)))

(fn ConstructionScript)