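; BP_Checkpoint is a checkpoint actor that records a respawn-style saved location for the third-person character.
; When its Box is overlapped by BP_ThirdPersonCharacter, it writes its own actor location into that character's SavedLocation.
; It then applies the MTL_Stairs material to the pieces of a referenced Staircase and plays a 2D "tada" sound.
; Nothing guards against retriggering, so every qualifying overlap repeats the effect.
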(event OnComponentBeginOverlap(Box)
  (params (OverlappedComponent :type Primitive%20Component%20Object%20Reference) (OtherActor :type Actor%20Object%20Reference) (OtherComp :type Primitive%20Component%20Object%20Reference) (OtherBodyIndex :type Integer) (bFromSweep :type Boolean) (SweepResult :type Hit%20Result%20Structure%20%28by%20ref%29))
  (bind _asbp_third_person_character (Utilities|Casting|CastToBP_ThirdPersonCharacter OtherActor))
  (Variables|/Game/ThirdPerson/Blueprints/BP_ThirdPersonCharacter.BP_ThirdPersonCharacter_C|SetSavedLocation _asbp_third_person_character (Transformation|GetActorLocation))
  (Rendering|Material|SetMaterial (Variables|/Game/Blueprints/BP_Staircase.BP_Staircase_C|GetStaircase (Variables|Default|GetStaircase)) 0 "/Game/Material/MTL_Stairs.MTL_Stairs")
  (Audio|PlaySound2D "/Game/Sounds/TadaSound.TadaSound" 1.0 1.0 0.0 0 0))

(event EventBeginPlay)

(event Collision|EventActorBeginOverlap
  (params (OtherActor :type Actor%20Object%20Reference)))

(event EventTick
  (params (DeltaSeconds :type Float%20%28single-precision%29)))

(fn ConstructionScript)